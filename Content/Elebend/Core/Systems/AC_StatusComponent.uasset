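; AC_StatusComponent is a component that tracks the active statuses on its owner.
; ApplyStatus adds a status to the ActiveStatus collection and fires the OnStatusApplied dispatcher, while RemoveStatus removes one after a HasStatus check.
; On BeginPlay it binds to its own dispatcher and prints every active status whenever one is applied, as debug output.
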(event `self.ReceiveBeginPlay`
  (add `self.onStatusApplied` (delegate `CustomEvent`)))

(event `CustomEvent` :!signature `self.onStatusApplied`
  (params (statusApplied :type "/Game/Elebend/Core/Elements/ENUM_Status Enum" :default "NewEnumerator0"))
  (for _array_element (`self.activeStatus`)
    (`KismetSystemLibrary.PrintString` (`|GetEnumeratorNameAsString` _array_element))))

(fn `applyStatus`
  (params (status :type "/Game/Elebend/Core/Elements/ENUM_Status Enum" :default "NewEnumerator0"))
  (`KismetArrayLibrary.Array_Add` (`self.activeStatus`) status)
  (`self.onStatusApplied` status))

(fn `hasStatus`
  (params (status :type "/Game/Elebend/Core/Elements/ENUM_Status Enum" :default "NewEnumerator0"))
  (returns (hasStatus :type Boolean))
  (locals (NewLocalVar :type "Array of String"))
  (for _array_element (`self.activeStatus`)
    (if (`|EnumEquality` _array_element status)
      (return true))))

(fn `removeStatus`
  (params (status :type "/Game/Elebend/Core/Elements/ENUM_Status Enum" :default "NewEnumerator0"))
  (bind _hasstatus (`self.hasStatus` status))
  (if _hasstatus
    (`KismetArrayLibrary.Array_RemoveItem` (`self.activeStatus`) status)))