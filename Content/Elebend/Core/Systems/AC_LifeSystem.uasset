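; AC_LifeSystem is a component, by its name, that tracks an actor's lives or health.
; SetFullLifes refills to MaxLife, while Heal and Damage add to or subtract from CurrentLifes.
; Each change fires OnLifeChanged, and Damage also fires OnDeath when the value drops to zero or below.
; The value is never clamped, so healing can exceed the maximum and repeated damage can retrigger death.
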(fn `damage`
  (params (damageValue :type Integer))
  (bind _output_get (set `self.currentLifes` (- (`self.currentLifes`) damageValue)))
  (`self.onLifeChanged`)
  (if (<= _output_get 0)
    (`self.onDeath`)))

(fn `heal`
  (params (healValue :type Integer))
  (set `self.currentLifes` (+ (`self.currentLifes`) healValue))
  (`self.onLifeChanged`))

(fn `setFullLifes`
  (set `self.currentLifes` (`self.maxLife`))
  (`self.onLifeChanged`))